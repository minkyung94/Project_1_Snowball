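; BP_Snowball is a rolling snowball actor that grows with the player character's state and bursts on a timer.
; Tick lerps its scale from normal to double using MoveSnowballScale from BP_ThirdPersonCharacter and spins the Snowball component around relative roll at RotationSpeed.
; BeginPlay starts a fixed-delay lifetime: it spawns an emitter and sound, hides the Snowball component, then destroys the actor after another delay.
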(event Collision|EventActorBeginOverlap
  (params (OtherActor :type Actor%20Object%20Reference)))

(event EventTick
  (params (DeltaSeconds :type Float%20%28single-precision%29))
  ;[1 1 1] 눈덩이 점점 커지게
  (bind _asbp_third_person_character (Utilities|Casting|CastToBP_ThirdPersonCharacter (Game|GetPlayerCharacter 0)))
  (Transformation|SetActorScale3D (Math|Vector|Lerp(Vector) (Math|Vector|MakeVector 1.0 1.0 1.0) (Math|Vector|MakeVector 2.0 2.0 2.0) (Variables|/Game/Blueprints/BP_ThirdPersonCharacter.BP_ThirdPersonCharacter_C|GetMoveSnowballScale _asbp_third_person_character)))
  ;[1 1 1] 눈덩이 회전 플레이어 기준 앞으로
  (Transformation|AddRelativeRotation (Variables|Default|GetSnowball) (Math|Rotator|MakeRotator (* (Utilities|Time|GetWorldDeltaSeconds) (Variables|Default|GetRotation%20Speed)) 0.0 0.0) false false))

(event EventBeginPlay
  ;[1 1 1] 눈덩이 발사할 때
  (Utilities|FlowControl|Delay 5.0)
  (Effects|SpawnEmitteratLocation 0 (Transformation|GetActorLocation) "0, 0, 0" "2.000000,1.000000,1.000000")
  (Audio|PlaySoundatLocation 0 (Transformation|GetActorLocation) "0, 0, 0" 1.0 1.0 0.0 0 0 0 0)
  (Development|SetHiddeninGame (Variables|Default|GetSnowball) true false)
  (Utilities|FlowControl|Delay 3.0)
  (Actor|DestroyActor))

(fn ConstructionScript)

(fn NewFunction)