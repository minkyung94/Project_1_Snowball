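; BP_Snowball is a snowball actor tied to the third-person character that grows and rolls until it is launched.
; While physics is off, Tick rolls the mesh by actor velocity and, unless IsLaunched is set, lerps actor scale up to double using the character's MoveSnowballScale.
; Launch enables physics simulation and applies the given force as a velocity-change impulse, which stops the Tick-driven growth and roll.
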(event Custom|Launch
  (params (Force :type Vector))
  (bind _snowball (Variables|Default|GetSnowball))
  ;[1 1 1] 발사
  (Physics|SetSimulatePhysics _snowball true)
  (Physics|AddImpulse _snowball Force "None" true))

(event EventBeginPlay
  ;[1 1 1] Comment
  (bind _returnvalue (Actor|GetActorOfClass "/Game/Blueprints/BP_ThirdPersonCharacter.BP_ThirdPersonCharacter_C"))
  (Variables|Default|SetOwningCharcter _returnvalue))

(event EventTick
  (params (DeltaSeconds :type Float%20%28single-precision%29))
  (if (not (Physics|IsSimulatingPhysics (Variables|Default|GetSnowball) "None"))
    ;[1 1 1] 눈덩이 2배 커지는 함수
    (CallFunction|MakeSnowballBigger)))

(fn ConstructionScript)

(fn MakeSnowballBigger
  ;[1 1 1] 눈덩이 점점 커지게 Lerp (2배 커지게)
  (if (Variables|Default|GetIsLaunched?)
    _
    (else
      (Transformation|SetActorScale3D (Math|Vector|Lerp(Vector) (Math|Vector|MakeVector 1.0 1.0 1.0) (Math|Vector|MakeVector 2.0 2.0 2.0) (Variables|/Game/Blueprints/BP_ThirdPersonCharacter.BP_ThirdPersonCharacter_C|GetMoveSnowballScale (Variables|Default|GetOwningCharcter))))
      ;[1 1 1] x 축이 플레이어 앞으로
      (bind _snowball (Variables|Default|GetSnowBall)
        (:then
          _)
        (:else))))
  (Transformation|AddLocalRotation _snowball (Math|Rotator|MakeRotator (* (Math|Vector|VectorLength (Transformation|GetVelocity)) (Utilities|Time|GetWorldDeltaSeconds) 1.0) 0.0 0.0) false false))