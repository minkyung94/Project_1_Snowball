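; Snowball actor that grows and spins until it is launched from the third-person character.
; Each Tick before launch, it lerps its scale up to double using the character's MoveSnowballScale and rotates the mesh.
; Launch releases the owner reference, enables physics and fires an impulse along the character's forward vector.
; Trigger-overlap, delayed burst effect and manual-movement logic are unconnected, and Tick still prints a physics debug string.
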(event Custom|Launch
  (Variables|Default|SetLaunchDIrection (Transformation|GetActorForwardVector (Variables|Default|GetOwningCharcter)))
  (Variables|Default|SetIsLaunched? true)
  (Variables|Default|SetOwningCharcter 0)
  (Physics|SetSimulatePhysics (Variables|Default|GetSnowball) true)
  (Physics|AddImpulse (Variables|Default|GetSnowball) (* (Variables|Default|GetLaunchDIrection) (Variables|Default|GetLaunchSpeed)) "None" false))

(event Collision|EventActorBeginOverlap
  (params (OtherActor :type Actor%20Object%20Reference)))

(event EventBeginPlay
  (bind _returnvalue (Actor|GetActorOfClass "/Game/Blueprints/BP_ThirdPersonCharacter.BP_ThirdPersonCharacter_C"))
  (Variables|Default|SetOwningCharcter _returnvalue))

(event EventTick
  (params (DeltaSeconds :type Float%20%28single-precision%29))
  (Development|PrintString (Utilities|String|ToString(Boolean) (Physics|IsSimulatingPhysics (Variables|Default|GetSnowball) "None")))
  (if (not (Variables|Default|GetIsLaunched?))
    ;[1 1 1] 눈덩이 2배 커지는 함수
    (CallFunction|MakeSnowballBigger)))

(fn ConstructionScript)

(fn MakeSnowballBigger
  ;[1 1 1] 눈덩이 점점 커지게 Lerp (2배 커지게)
  (if (Variables|Default|GetIsLaunched?)
    _
    (else
      (Transformation|SetActorScale3D (Math|Vector|Lerp(Vector) (Math|Vector|MakeVector 1.0 1.0 1.0) (Math|Vector|MakeVector 2.0 2.0 2.0) (Variables|/Game/Blueprints/BP_ThirdPersonCharacter.BP_ThirdPersonCharacter_C|GetMoveSnowballScale (Variables|Default|GetOwningCharcter))))))
  ;[1 1 1] 눈덩이 회전 플레이어 기준 앞으로
  (Transformation|AddRelativeRotation (Variables|Default|GetSnowball) (Math|Rotator|MakeRotator (* (Utilities|Time|GetWorldDeltaSeconds) (Variables|Default|GetRotation%20Speed)) 0.0 0.0) false false))